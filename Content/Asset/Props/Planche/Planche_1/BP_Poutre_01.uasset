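; Beam prop that pitches into a new position once it has received the required number of ActivateObject calls, only the first time.
; A timeline rotates the scene component, scaled by RotationYRelative, with beam collision disabled during the motion.
; When it finishes, collision returns and Pousse repeatedly shoves the player capsule backward along its forward vector after short delays, while it overlaps the Box.
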(event `/Game/BP/Briques_De_Jeu/BPI_ActivateObject.ActivateObject`
  (bind _output_get (set `self.nb temp` (+ (`self.nb temp`) 1)))
  (if (== _output_get (`self.nb to activate`))
    (`/Engine/EditorBlueprintResources/StandardMacros.DoOnce` false
      (:`Completed`
        (`PrimitiveComponent.SetCollisionEnabled` (`self.Poutre`) "NoCollision")
        (bind (_direction _rotation) (`Timeline|Timeline` :!via `PlayFromStart`)
          (:`Update`
            (`SceneComponent.K2_SetRelativeRotation` (`self.ScenePoutre`) (`KismetMathLibrary.MakeRotator` 0.0 (* (.y _rotation) (`self.Rotation Y relative`))) false false))
          (:`Finished`
            (`PrimitiveComponent.SetCollisionEnabled` (`self.Poutre`) "QueryAndPhysics")
            (`self.Pousse`)))))))

(event `Pousse`
  (`KismetSystemLibrary.Delay` 0.1)
  (bind _asbp_player (cast `/Game/BP/BP_Player` (`GameplayStatics.GetPlayerPawn` 0)))
  (bind _capsule (`/Game/BP/BP_Player.Capsule` _asbp_player))
  (if (`PrimitiveComponent.IsOverlappingComponent` (`self.Box`) _capsule)
    (`PrimitiveComponent.AddVelocityChangeImpulseAtLocation` _capsule (* (`SceneComponent.GetForwardVector` _capsule) -1000.0) (`SceneComponent.K2_GetComponentLocation` _capsule) "None")
    (`self.Pousse`)))

(fn `UserConstructionScript`)