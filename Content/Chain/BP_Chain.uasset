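; BP_Chain is a chain actor with a physics ball (Boulet) whose damping changes between falling and resting on the floor.
; It caches the ball's linear and angular damping at BeginPlay and applies DampingInAir to both when falling.
; A 0.01-second timer repeats a downward sphere trace, ignoring BP_Chain hits, and restores the cached damping within 40 units of a hit.
; Mass override nodes are present but unconnected.
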(event `self.ReceiveBeginPlay`
  (bind _boulet (`self.Boulet`))
  (set `self.Boulet Linear damping` (`PrimitiveComponent.GetLinearDamping` _boulet))
  (set `self.Boulet Angular Damping` (`PrimitiveComponent.GetAngularDamping` _boulet)))

(event `Set Parameter When On Floor`
  (bind _boulet (`self.Boulet`))
  (`PrimitiveComponent.SetLinearDamping` _boulet (`self.Boulet Linear damping`))
  (`PrimitiveComponent.SetAngularDamping` _boulet (`self.Boulet Angular Damping`)))

(event `Set Parameter When Falling`
  (bind _damping_in_air (`self.Damping In Air`))
  (bind _boulet (`self.Boulet`))
  (`PrimitiveComponent.SetLinearDamping` _boulet _damping_in_air)
  (`PrimitiveComponent.SetAngularDamping` _boulet _damping_in_air)
  (`self.CheckBouletHeigh`))

(event `CheckBouletHeigh`
  (bind _boulet (`self.Boulet`))
  (bind (_returnvalue_x _returnvalue_y _returnvalue_z) (`KismetMathLibrary.BreakVector` (`SceneComponent.K2_GetComponentLocation` _boulet)))
  (bind _returnvalue (`KismetSystemLibrary.K2_SetTimerDelegate` (delegate `CheckBouletHeigh`) 0.01 true))
  (set `self.Heigh Boulet Event` _returnvalue)
  (bind _outhit (`KismetSystemLibrary.SphereTraceSingle` (`SceneComponent.K2_GetComponentLocation` _boulet) (`KismetMathLibrary.MakeVector` _returnvalue_x _returnvalue_y (- _returnvalue_z 2000.0)) 5.0 "TraceTypeQuery1"))
  (cast `/Game/Chain/BP_Chain` (`.HitActor` (`GameplayStatics.BreakHitResult` _outhit))
    (:`CastFailed`
      (if (< (`.Distance` (`GameplayStatics.BreakHitResult` _outhit)) 40.0)
        (`self.Set Parameter When On Floor`)
        (`KismetSystemLibrary.K2_ClearAndInvalidateTimerHandle` (`self.Heigh Boulet Event`))))))

(fn `UserConstructionScript`)