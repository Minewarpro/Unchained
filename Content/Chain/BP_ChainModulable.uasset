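; BP_ChainModulable is a configurable physics ball and chain, with a link count, spacing, scale and total weight.
; The construction script spawns links with alternating roll, joins them with physics constraints to the ball (Boulet), and splits the weight evenly; SetPoidChains redistributes it.
; SetParameterWhenFalling switches the ball to in-air damping and starts a timed downward sphere trace that restores its original damping near the floor.
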(event `self.ReceiveBeginPlay`
  (bind _boulet (`self.Boulet`))
  (set `self.Boulet Linear damping` (`PrimitiveComponent.GetLinearDamping` _boulet))
  (set `self.Boulet Angular Damping` (`PrimitiveComponent.GetAngularDamping` _boulet)))

(event `Set Parameter When On Floor`
  (bind _boulet (`self.Boulet`))
  (`PrimitiveComponent.SetLinearDamping` _boulet (`self.Boulet Linear damping`))
  (`PrimitiveComponent.SetAngularDamping` _boulet (`self.Boulet Angular Damping`)))

(event `Set Parameter When Falling`
  (bind _damping_in_air (`self.Damping In Air`))
  (bind _boulet (`self.Boulet`))
  (`PrimitiveComponent.SetLinearDamping` _boulet _damping_in_air)
  (`PrimitiveComponent.SetAngularDamping` _boulet _damping_in_air)
  (`self.CheckBouletHeigh`))

(event `CheckBouletHeigh`
  (bind _boulet (`self.Boulet`))
  (bind (_returnvalue_x _returnvalue_y _returnvalue_z) (`KismetMathLibrary.BreakVector` (`SceneComponent.K2_GetComponentLocation` _boulet)))
  (bind _returnvalue (`KismetSystemLibrary.K2_SetTimerDelegate` (delegate `CheckBouletHeigh`) 0.01 true))
  (set `self.Heigh Boulet Event` _returnvalue)
  (bind _outhit (`KismetSystemLibrary.SphereTraceSingle` (`SceneComponent.K2_GetComponentLocation` _boulet) (`KismetMathLibrary.MakeVector` _returnvalue_x _returnvalue_y (- _returnvalue_z 2000.0)) 5.0 "TraceTypeQuery1"))
  (cast `/Game/Chain/BP_ChainModulable` (`.HitActor` (`GameplayStatics.BreakHitResult` _outhit))
    (:`CastFailed`
      (if (< (`.Distance` (`GameplayStatics.BreakHitResult` _outhit)) 40.0)
        (`self.Set Parameter When On Floor`)
        (`KismetSystemLibrary.K2_ClearAndInvalidateTimerHandle` (`self.Heigh Boulet Event`))))))

(fn `SetPoidChains`
  (params (NouveauPoids :type "Float (double-precision)"))
  (for _array_element (`self.MaillonArray`)
    (`PrimitiveComponent.SetMassOverrideInKg` _array_element "None" (/ NouveauPoids (`KismetArrayLibrary.Array_Length` (`self.MaillonArray`))) true)))

(fn `UserConstructionScript`
  (locals (MaillonXPos :type "Float (double-precision)" :default 0.0) (MaillonXRol :type "Float (single-precision)" :default 0.0))
  (bind _maillonarray (`self.MaillonArray`))
  (bind _maillonarray_2 (`self.MaillonArray`))
  (for _ (range (`self.NombreMaillons`))
    (set `local.MaillonXPos` (- (`local.MaillonXPos`) (`self.MaillonEcart`)))
    (`/Engine/EditorBlueprintResources/StandardMacros.FlipFlop`
      (:`A`
        (set `local.MaillonXRol` 0.0))
      (:`B`
        (set `local.MaillonXRol` 90.0)))
    (bind _returnvalue (`AddComponent|NODE_AddStaticMeshComponent-1` :`RelativeTransform` (`KismetMathLibrary.MakeTransform` (`KismetMathLibrary.MakeVector` (`local.MaillonXPos`)) (`KismetMathLibrary.MakeRotator` (`local.MaillonXRol`)) (`KismetMathLibrary.Conv_DoubleToVector` (`self.ScaleMaillon`)))))
    (`PrimitiveComponent.SetMassOverrideInKg` _returnvalue "None" (/ (`self.PoidTotalChaine`) (`self.NombreMaillons`)) true)
    (`KismetArrayLibrary.Array_Add` (`self.MaillonArray`) _returnvalue)
    (bind _returnvalue_2 (`AddComponent|NODE_AddPhysicsConstraintComponent-0` :`RelativeTransform` (`KismetMathLibrary.MakeTransform` (`KismetMathLibrary.MakeVector` (`local.MaillonXPos`)))))
    (if (> (`KismetArrayLibrary.Array_Length` (`self.MaillonArray`)) 1)
      (`PhysicsConstraintComponent.SetConstrainedComponents` _returnvalue_2 (`|GetArrayItem` _maillonarray_2 (- (`KismetArrayLibrary.Array_LastIndex` _maillonarray_2) 1)) "None" (`|GetArrayItem` _maillonarray_2 (`KismetArrayLibrary.Array_LastIndex` _maillonarray_2)) "None")))
  (bind _returnvalue_3 (`AddComponent|NODE_AddPhysicsConstraintComponent-2` :`RelativeTransform` (`KismetMathLibrary.MakeTransform` (`KismetMathLibrary.MakeVector` (- (`local.MaillonXPos`) 10.0)))))
  (`PhysicsConstraintComponent.SetConstrainedComponents` _returnvalue_3 (`self.Boulet`) "None" (`|GetArrayItem` _maillonarray (`KismetArrayLibrary.Array_LastIndex` _maillonarray)) "None"))