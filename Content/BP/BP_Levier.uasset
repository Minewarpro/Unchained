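; Lever Blueprint that, when interacted with, moves its Torch01 component vertically and unlocks a linked object.
; Interact plays the Activate timeline, whose Height track scaled by Disctance offsets the torch from the actor Z cached at BeginPlay.
; Each timeline update, rather than its completion, also sets CanOpen on ObjectToActivate and calls its InteractMessage, so that call repeats throughout the animation.
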(event `self.ReceiveBeginPlay`
  (bind (_returnvalue_x _returnvalue_y _returnvalue_z) (`KismetMathLibrary.BreakVector` (`self.K2_GetActorLocation`)))
  (set `self.Location_Z` _returnvalue_z))

(event `/Game/BP/BPI_Interact.Interact`
  (params (Player :type "/Game/FirstPerson/Blueprints/BP_FirstPersonCharacter Object Reference"))
  (bind (_returnvalue_x _returnvalue_y _returnvalue_z) (`KismetMathLibrary.BreakVector` (`self.K2_GetActorLocation`)))
  (bind _objecttoactivate (`self.ObjectToActivate`))
  (bind (_direction _height) (`Timeline|Activate`)
    (:`Update`
      (`SceneComponent.K2_SetWorldLocation` (`self.Torch_01`) (`KismetMathLibrary.MakeVector` _returnvalue_x _returnvalue_y (+ (* _height (`self.Disctance`)) (`self.Location_Z`))) false false)
      (set `/Game/BP/BP_Door.CanOpen` true _objecttoactivate)
      (message `/Game/BP/BPI_Interact.Interact` _objecttoactivate null))))

(fn `UserConstructionScript`)