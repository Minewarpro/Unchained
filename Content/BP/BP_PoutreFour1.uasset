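; Activatable beam Blueprint (PoutreFour1) that rotates its static mesh to a target rotation, one time only.
; ActivateObject records the mesh's current world rotation, then plays the Deplacement timeline through a DoOnce.
; The timeline's Location vector serves as separate roll, pitch and yaw alphas, interpolating from the recorded rotation toward RotationTo.
; When the timeline finishes, it prints the final rotation.
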(event `/Game/BP/Briques_De_Jeu/BPI_ActivateObject.ActivateObject`
  (bind (_rotationto_roll _rotationto_pitch _rotationto_yaw) (`KismetMathLibrary.BreakRotator` (`self.RotationTo`)))
  (bind (_initworldrotation_roll _initworldrotation_pitch _initworldrotation_yaw) (`KismetMathLibrary.BreakRotator` (`self.InitWorldRotation`)))
  (bind (_initworldrotation_roll_2 _initworldrotation_pitch_2 _initworldrotation_yaw_2) (`KismetMathLibrary.BreakRotator` (`self.InitWorldRotation`)))
  (set `self.InitWorldRotation` (`SceneComponent.K2_GetComponentRotation` (`self.StaticMesh`)))
  (`/Engine/EditorBlueprintResources/StandardMacros.DoOnce` false
    (:`Completed`
      (bind (_direction _location) (`Timeline|Deplacement` :!via `PlayFromStart`)
        (:`Update`
          (`SceneComponent.K2_SetWorldRotation` (`self.StaticMesh`) (`KismetMathLibrary.MakeRotator` (+ (* (.x _location) (- _rotationto_roll _initworldrotation_roll_2)) _initworldrotation_roll) (+ (* (.y _location) (- _rotationto_pitch _initworldrotation_pitch_2)) _initworldrotation_pitch) (+ (* (.z _location) (- _rotationto_yaw _initworldrotation_yaw_2)) _initworldrotation_yaw)) false false))
        (:`Finished`
          (`KismetSystemLibrary.PrintString` (`KismetStringLibrary.Conv_RotatorToString` (`SceneComponent.K2_GetComponentRotation` (`self.StaticMesh`)))))))))

(fn `UserConstructionScript`)