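; Respawn point actor that becomes active when the player reaches it.
; A DetectionSphere is sized from SphereRadius at BeginPlay, and the first overlap by player pawn 0 sets IsEnable through a DoOnce and prints a message.
; GetIsEnable exposes that state, and Tick can draw a debug sphere of the detection radius.
; The file itself holds no respawn logic.
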(event `self.ReceiveBeginPlay`
  (`SphereComponent.SetSphereRadius` (`self.DetectionSphere`) (`self.SphereRadius`) true))

(event `self.ReceiveActorBeginOverlap`
  (params (OtherActor :type "Actor Object Reference"))
  (if (== OtherActor (`GameplayStatics.GetPlayerPawn` 0))
    (`/Engine/EditorBlueprintResources/StandardMacros.DoOnce` false
      (:`Completed`
        (set `self.IsEnable` true)
        (`KismetSystemLibrary.PrintString` "SPAWN IS ACTIVATED")))))

(event `self.ReceiveTick`
  (params (DeltaSeconds :type "Float (single-precision)"))
  (if (`self.DrawDebugSphere`)
    (`KismetSystemLibrary.DrawDebugSphere` (`self.K2_GetActorLocation`) (`self.SphereRadius`) 12 (struct :`R` 1.0 :`B` 0.068288 :`A` 1.0) 0.0 2.0)))

(fn `GetIsEnable`
  (returns (IsEnable :type Boolean))
  (return (`self.IsEnable`)))

(fn `UserConstructionScript`)