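; BP_Door is an interactable door actor that slides vertically open when Interact is called and CanOpen is set.
; On BeginPlay it stores its starting Z height.
; Interact plays the Open timeline, whose curve scales Distance and adds it to that height to move the actor with sweep enabled.
; The graph contains no closing logic.
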(event `self.ReceiveBeginPlay`
  (bind (_returnvalue_x _returnvalue_y _returnvalue_z) (`KismetMathLibrary.BreakVector` (`self.K2_GetActorLocation`)))
  (set `self.Location_Z` _returnvalue_z))

(event `/Game/BP/BPI_Interact.Interact`
  (params (Player :type "/Game/FirstPerson/Blueprints/BP_FirstPersonCharacter Object Reference"))
  (bind (_returnvalue_x _returnvalue_y _returnvalue_z) (`KismetMathLibrary.BreakVector` (`self.K2_GetActorLocation`)))
  (if (`self.CanOpen`)
    (bind (_direction _openanimation) (`Timeline|Open`)
      (:`Update`
        (`self.K2_SetActorLocation` (`KismetMathLibrary.MakeVector` _returnvalue_x _returnvalue_y (+ (* _openanimation (`self.Distance`)) (`self.Location_Z`))) true)))))

(fn `UserConstructionScript`)