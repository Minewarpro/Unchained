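; Player camera Blueprint that randomly shows or hides the BP_MonsterMenue actor when something, apparently a ball, passes in front of it.
; A looping timer sphere-traces from the camera to a point above the monster against one object type.
; Each new blocking hit rolls to toggle visibility, so the swap happens while the view is obstructed.
; The odds shift with state, making the monster quicker to vanish than to reappear.
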(event `self.ReceiveBeginPlay`
  (bind _returnvalue (`GameplayStatics.GetActorOfClass` "/Game/BP/BP_MonsterMenue.BP_MonsterMenue_C"))
  (set `self.TargetLineTrace` _returnvalue)
  (`KismetSystemLibrary.K2_SetTimerDelegate` (delegate `TraceDetection`) 0.1 true)
  (`self.TraceDetection`))

(event `TraceDetection`
  (bind _outhit (`KismetSystemLibrary.SphereTraceSingleForObjects` :`Start` (`SceneComponent.K2_GetComponentLocation` (`self.Camera`)) :`End` (+ (`self.K2_GetActorLocation` (`self.TargetLineTrace`)) (0.0 0.0 390.0)) :`Radius` 1.0 :`ObjectTypes` (`|MakeArray` "ObjectTypeQuery8" :!type "EObjectTypeQuery Enum") :`DrawTime` 0.1))
  (if (`GameplayStatics.BreakHitResult` _outhit)
    (if (not (`self.IsBallInFront`))
      (set `self.IsBallInFront` true)
      (if (== (`KismetMathLibrary.RandomInteger` (`self.MaxRandom`)) 0)
        (bind _output_get (set `self.IsHidden` (not (`self.IsHidden`))))
        (`self.SetActorHiddenInGame` (`self.TargetLineTrace`) _output_get)
        (if (`self.IsHidden`)
          (set `self.MaxRandom` 6)
          (else
            (set `self.MaxRandom` 2)))))
    (else
      (set `self.IsBallInFront` false))))

(fn `UserConstructionScript`)