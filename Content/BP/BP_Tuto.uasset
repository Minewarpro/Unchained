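; BP_Tuto is a trigger box that shows a numbered tutorial step when the player walks into it.
; On overlap it checks that the other actor is BP_Player and the touching component is its capsule, then fires once through a DoOnce.
; The NbTuto variable selects which of the player's Tuto02, Tuto03 or Tuto04 functions runs, so the tutorial logic itself lives in BP_Player.
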(event `self.Box.OnComponentBeginOverlap`
  (params (OverlappedComponent :type "PrimitiveComponent Object Reference") (OtherActor :type "Actor Object Reference") (OtherComp :type "PrimitiveComponent Object Reference") (OtherBodyIndex :type Integer) (bFromSweep :type Boolean) (SweepResult :type "HitResult Structure (by ref)"))
  (bind _asbp_player (cast `/Game/BP/BP_Player` OtherActor))
  (if (== OtherComp (`/Game/BP/BP_Player.Capsule` _asbp_player))
    (`/Engine/EditorBlueprintResources/StandardMacros.DoOnce` false
      (:`Completed`
        (if (== (`self.Nb Tuto`) 2)
          (`/Game/BP/BP_Player.Tuto_02` _asbp_player)
          (elif (== (`self.Nb Tuto`) 3)
            (`/Game/BP/BP_Player.Tuto_03` _asbp_player)
            (elif (== (`self.Nb Tuto`) 4)
              (`/Game/BP/BP_Player.Tuto_04` _asbp_player))))))))

(fn `UserConstructionScript`)