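; BP_ActivableBox is a trigger volume, box or sphere as chosen in the construction script, that fires scripted events when BP_Player overlaps it.
; Overlap activates a target object once after a delay, with optional light reveal, sound and camera shake.
; An optional one-shot sequence locks input and blends cameras, then repositions the player, swapping chain for rope.
; An optional delayed call resets the BP_NPC chase.
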(event `PlaySequence`
  (bind _returnvalue (`GameplayStatics.GetPlayerController` 0))
  (bind _as_bp_player (`self.As BP Player`))
  (bind _as_bp_player_2 (`self.As BP Player`))
  (bind _as_bp_player_3 (`self.As BP Player`))
  (bind _sequenceplayer (`LevelSequenceActor.SequencePlayer` (`self.Sequencer to play`)))
  (bind _returnvalue_2 (`TimeManagementBlueprintLibrary.Conv_QualifiedFrameTimeToSeconds` (`MovieSceneSequencePlayer.GetDuration` _sequenceplayer)))
  (if (`self.Need sequencer`)
    (`/Engine/EditorBlueprintResources/StandardMacros.DoOnce` false
      (:`Completed`
        (set `/Game/BP/BP_Player.IsBouletBroken` true _as_bp_player_2)
        (set `/Game/BP/BP_Player.IsInpoutMovePress` false _as_bp_player_2)
        (`/Game/BP/BP_Player.Stop walking` _as_bp_player_2)
        (`self.DisableInput` _as_bp_player_2 _returnvalue)
        (bind _output_get (set `self.Cam to return` (`Controller.GetViewTarget` _returnvalue)))
        (`KismetSystemLibrary.PrintString` (`KismetSystemLibrary.GetDisplayName` _output_get))
        (`PlayerController.SetViewTargetWithBlend` _returnvalue (`self.Cam to blend`) (`self.Blend Time`) "VTBlend_Linear" 0.0 false)
        (`MovieSceneSequencePlayer.Play` _sequenceplayer)
        (`|ExecutionSequence`
          (:`then_0`
            (`KismetSystemLibrary.Delay` _returnvalue_2)
            (`/Game/BP/BP_Player.Destroy Chain` _as_bp_player_3)
            (`self.K2_SetActorLocation` _as_bp_player_3 (`self.New Location`) false false)
            (`Controller.SetControlRotation` (`Pawn.GetController` (`Actor.Instigator` _as_bp_player_3)) (`self.New Rotation`))
            (`/Game/BP/BP_Player.SpawnRope` _as_bp_player_3)
            (`SceneComponent.K2_SetRelativeLocation` (`/Game/BP/BP_Player.Camera` _as_bp_player_3) (-10.0 0.0 45.0) false true)
            (`PlayerController.SetViewTargetWithBlend` (`GameplayStatics.GetPlayerController` 0) (`self.Cam to return`) (`self.Blend Time`) "VTBlend_Linear" 0.0 false)
            (`self.EnableInput` _as_bp_player (`GameplayStatics.GetPlayerController` 0))
            (set `/Game/BP/BP_Player.IsBouletBroken` false _as_bp_player))
          (:`then_1`
            (`KismetSystemLibrary.Delay` (- _returnvalue_2 0.1))
            (set `self.New Rotation` (`self.K2_GetActorRotation` (`self.Cam to blend`)))))))))

(event `Activate Box`
  (params (B :type "Object Object Reference"))
  (bind (_returnvalue_x _returnvalue_y _returnvalue_z) (`KismetMathLibrary.BreakVector` (`self.K2_GetActorLocation`)))
  (bind _light_to_activate (`self.Light To activate`))
  (`/Engine/EditorBlueprintResources/StandardMacros.DoOnce` false
    (:`Completed`
      (`KismetSystemLibrary.Delay` (`self.delay`))
      (message `/Game/BP/Briques_De_Jeu/BPI_ActivateObject.ActivateObject` (`self.Object To Activate`))
      (`/Engine/EditorBlueprintResources/StandardMacros.IsValid` _light_to_activate
        (:`Is Valid`
          (`self.SetActorHiddenInGame` _light_to_activate false))
        (:`Is Not Valid`
          _))
      (`GameplayStatics.PlaySoundAtLocation` (`self.Sound`) (`KismetMathLibrary.MakeVector` _returnvalue_x _returnvalue_y (+ _returnvalue_z 1400.0)) (struct) 1.0 1.0 0.0 null null null null)
      (`PlayerCameraManager.StartCameraShake` :`self` (`GameplayStatics.GetPlayerCameraManager` 0) :`ShakeClass` (`self.Shake Class`)))))

(event `self.Sphere.OnComponentBeginOverlap`
  (params (OverlappedComponent :type "PrimitiveComponent Object Reference") (OtherActor :type "Actor Object Reference") (OtherComp :type "PrimitiveComponent Object Reference") (OtherBodyIndex :type Integer) (bFromSweep :type Boolean) (SweepResult :type "HitResult Structure (by ref)"))
  (bind _asbp_player (cast `/Game/BP/BP_Player` OtherActor))
  (set `self.As BP Player` _asbp_player)
  (`self.Activate Box` null)
  (`self.PlaySequence`)
  (`self.reset chase`))

(event `self.Box.OnComponentBeginOverlap`
  (params (OverlappedComponent :type "PrimitiveComponent Object Reference") (OtherActor :type "Actor Object Reference") (OtherComp :type "PrimitiveComponent Object Reference") (OtherBodyIndex :type Integer) (bFromSweep :type Boolean) (SweepResult :type "HitResult Structure (by ref)"))
  (bind _asbp_player (cast `/Game/BP/BP_Player` OtherActor))
  (set `self.As BP Player` _asbp_player)
  (`self.Activate Box` null)
  (`self.PlaySequence`)
  (`self.reset chase`))

(event `reset chase`
  (if (`self.need reset chase`)
    (`KismetSystemLibrary.Delay` (`self.delay reset chase`))
    (bind _returnvalue (`GameplayStatics.GetActorOfClass` "/Game/Characters/AI/BP_NPC.BP_NPC_C"))
    (`/Game/Characters/AI/BP_NPC.Reset Chase` _returnvalue)))

(fn `UserConstructionScript`
  (bind _sphere (`self.Sphere`))
  (bind _box (`self.Box`))
  (bind _sphere_2 (`self.Sphere`))
  (bind _box_2 (`self.Box`))
  (if (`self.Box Collider`)
    (`SceneComponent.SetVisibility` _box_2 true false)
    (`SceneComponent.SetVisibility` _sphere_2 false false)
    (set `PrimitiveComponent.bGenerateOverlapEvents` false _sphere_2)
    (set `PrimitiveComponent.bGenerateOverlapEvents` true _box_2)
    (else
      (`SceneComponent.SetVisibility` _box false false)
      (`SceneComponent.SetVisibility` _sphere true false)
      (set `PrimitiveComponent.bGenerateOverlapEvents` false _box)
      (set `PrimitiveComponent.bGenerateOverlapEvents` true _sphere))))