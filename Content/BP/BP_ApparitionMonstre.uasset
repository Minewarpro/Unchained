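; BP_ApparitionMonstre is an activatable actor that makes the monster NPC appear at its location.
; On BeginPlay it finds and caches the BP_NPC, AI_NPC and BP_Player actors; the construction script assigns its configurable Niagara effect.
; ActivateObject starts the effect and a camera shake, waits a configurable delay, then teleports the monster to the actor's root and optionally tells the AI to chase the player.
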(event `self.ReceiveBeginPlay`
  (bind _returnvalue (`GameplayStatics.GetActorOfClass` "/Game/Characters/AI/BP_NPC.BP_NPC_C"))
  (set `self.MonsterRef` _returnvalue)
  (bind _returnvalue_2 (`GameplayStatics.GetActorOfClass` "/Game/Characters/AI/AI_NPC.AI_NPC_C"))
  (set `self.As Ai` _returnvalue_2)
  (bind _returnvalue_3 (`GameplayStatics.GetActorOfClass` "/Game/BP/BP_Player.BP_Player_C"))
  (set `self.As Player` _returnvalue_3))

(event `/Game/BP/Briques_De_Jeu/BPI_ActivateObject.ActivateObject`
  (`ActorComponent.SetActive` (`self.Niagara1`) true false)
  (`PlayerCameraManager.StartCameraShake` :`self` (`GameplayStatics.GetPlayerCameraManager` 0) :`ShakeClass` (`self.Camera Shake Class`))
  (`KismetSystemLibrary.Delay` (`self.delay monstre apparition`))
  (`self.K2_SetActorLocation` (`self.MonsterRef`) (`SceneComponent.K2_GetComponentLocation` (`self.DefaultSceneRoot`)) false true)
  (if (`self.Need Target Player`)
    (`/Game/Characters/AI/AI_NPC.Chase Player` (`self.As Ai`))))

(fn `UserConstructionScript`
  (`NiagaraComponent.SetAsset` (`self.Niagara1`) (`self.Niagara`) true))