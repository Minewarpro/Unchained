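; Eye-blink intro actor that plays an opening cinematic on the game's first run when NeedSequence is set.
; BeginPlay adds an eyelid widget, then PlaySequencer disables input, blends to a cinematic camera and plays the sequence.
; Afterward it repositions the player with the camera's final rotation, swaps chain for rope, restores view and input, and starts the tutorial.
; A separate Ouvertureyeux event animates the eyelids and blur through a timeline, then removes the widget.
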(event `Play Sequencer`
  (bind _returnvalue (`GameplayStatics.GetPlayerController` 0))
  (bind _as_bp_player (`self.As BP Player`))
  (bind _as_bp_player_2 (`self.As BP Player`))
  (bind _as_bp_player_3 (`self.As BP Player`))
  (bind _sequenceplayer (`LevelSequenceActor.SequencePlayer` (`self.sequencer`)))
  (bind _returnvalue_2 (`TimeManagementBlueprintLibrary.Conv_QualifiedFrameTimeToSeconds` (`MovieSceneSequencePlayer.GetDuration` _sequenceplayer)))
  (`/Engine/EditorBlueprintResources/StandardMacros.DoOnce` false
    (:`Completed`
      (set `/Game/BP/BP_Player.IsBouletBroken` true _as_bp_player_2)
      (set `/Game/BP/BP_Player.IsInpoutMovePress` false _as_bp_player_2)
      (`/Game/BP/BP_Player.Stop walking` _as_bp_player_2)
      (`self.DisableInput` _as_bp_player_2 _returnvalue)
      (set `self.Cam to return` (`Controller.GetViewTarget` _returnvalue))
      (`PlayerController.SetViewTargetWithBlend` _returnvalue (`self.Cam to blend`) (`self.Blend Time`) "VTBlend_Linear" 0.0 false)
      (`MovieSceneSequencePlayer.Play` _sequenceplayer)
      (`|ExecutionSequence`
        (:`then_0`
          (`KismetSystemLibrary.Delay` _returnvalue_2)
          (`/Game/BP/BP_Player.Destroy Chain` _as_bp_player_3)
          (`self.K2_SetActorLocation` _as_bp_player_3 (`self.New Location`) false false)
          (`Controller.SetControlRotation` (`Pawn.GetController` (`Actor.Instigator` _as_bp_player_3)) (`self.New Rotation`))
          (`/Game/BP/BP_Player.SpawnRope` _as_bp_player_3)
          (`SceneComponent.K2_SetRelativeLocation` (`/Game/BP/BP_Player.Camera` _as_bp_player_3) (-10.0 0.0 45.0) false true)
          (`PlayerController.SetViewTargetWithBlend` (`GameplayStatics.GetPlayerController` 0) (`self.Cam to return`) (`self.Blend Time`) "VTBlend_Linear" 0.0 false)
          (`self.EnableInput` _as_bp_player (`GameplayStatics.GetPlayerController` 0))
          (set `/Game/BP/BP_Player.IsBouletBroken` false _as_bp_player)
          (bind _asbp_player (cast `/Game/BP/BP_Player` (`GameplayStatics.GetPlayerPawn` 0)))
          (`/Game/BP/BP_Player.StartTuto` _asbp_player))
        (:`then_1`
          (`KismetSystemLibrary.Delay` (- _returnvalue_2 0.1))
          (set `self.New Rotation` (`self.K2_GetActorRotation` (`self.Cam to blend`))))))))

(event `self.ReceiveBeginPlay`
  (if (`self.Need Sequence`)
    (bind _asbp_custom_game_instance (cast `/Game/BP/Briques_De_Jeu/BP_CustomGameInstance` (`GameplayStatics.GetGameInstance`)))
    (if (`/Game/BP/Briques_De_Jeu/BP_CustomGameInstance.IsFirstRun` _asbp_custom_game_instance)
      (bind _asbp_player (cast `/Game/BP/BP_Player` (`GameplayStatics.GetPlayerPawn` 0)))
      (set `self.As BP Player` _asbp_player)
      (bind _returnvalue (`|CreateWidget` "/Game/BP/ui/WB_Clignement.WB_Clignement_C"))
      (bind _output_get (set `self.Widget_Clignement_Ref` _returnvalue))
      (`UserWidget.AddToViewport` _output_get 0)
      (`Widget.SetRenderTranslation` (`/Game/BP/ui/WB_Clignement.Top` _output_get) (0.0 575.0))
      (`Widget.SetRenderTranslation` (`/Game/BP/ui/WB_Clignement.Bottom` _output_get) (0.0 -575.0))
      (`self.Play Sequencer`))))

(event `Ouverture yeux`
  (bind _widget_clignement_ref (`self.Widget_Clignement_Ref`))
  (`TimelineComponent.SetPlayRate` (`self.Ouverture`) (/ 1.0 3.0))
  (bind (_direction _translation_ _blur) (`Timeline|Ouverture` :!via `PlayFromStart`)
    (:`Update`
      (bind _returnvalue (* _translation_ 575.0))
      (`Widget.SetRenderTranslation` (`/Game/BP/ui/WB_Clignement.Top` _widget_clignement_ref) (`KismetMathLibrary.MakeVector2D` 0.0 _returnvalue))
      (`Widget.SetRenderTranslation` (`/Game/BP/ui/WB_Clignement.Bottom` _widget_clignement_ref) (`KismetMathLibrary.MakeVector2D` 0.0 (* _returnvalue -1.0)))
      (`BackgroundBlur.SetBlurStrength` (`/Game/BP/ui/WB_Clignement.Blur` _widget_clignement_ref) (* _blur 5.0)))
    (:`Finished`
      (`Widget.RemoveFromParent` (`self.Widget_Clignement_Ref`)))))

(fn `UserConstructionScript`)