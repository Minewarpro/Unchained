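; BP_pousiere is a dust effect actor that only keeps its Niagara particle component while the player is nearby.
; Each Tick compares the distance from its root to the BP_Player pawn cached at BeginPlay against a fixed radius.
; Entering range adds the component and sets its asset, while leaving destroys it.
; Two DoOnce nodes re-arm each other, so each transition fires once per crossing.
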(event `self.ReceiveBeginPlay`
  (bind _asbp_player (cast `/Game/BP/BP_Player` (`GameplayStatics.GetPlayerPawn` 0)))
  (set `self.Player Ref` _asbp_player))

(event `self.ReceiveTick`
  (params (DeltaSeconds :type "Float (single-precision)"))
  (if (< (`KismetMathLibrary.Vector_Distance` (`SceneComponent.K2_GetComponentLocation` (`self.DefaultSceneRoot`)) (`SceneComponent.K2_GetComponentLocation` (`Actor.RootComponent` (`self.Player Ref`)))) 1500.0)
    (`/Engine/EditorBlueprintResources/StandardMacros.DoOnce` false :!label _label
      (:`Completed`
        (bind _returnvalue (`AddComponent|NODE_AddNiagaraComponent-0`))
        (bind _output_get (set `self.particle` _returnvalue))
        (`NiagaraComponent.SetAsset` _output_get (`self.In Asset`) true)
        (goto _label_2 :!via `Reset`)))
    (else
      (`/Engine/EditorBlueprintResources/StandardMacros.IsValid` (`self.particle`)
        (:`Is Valid`
          (`/Engine/EditorBlueprintResources/StandardMacros.DoOnce` false :!label _label_2
            (:`Completed`
              (`ActorComponent.K2_DestroyComponent` (`self.particle`))
              (goto _label :!via `Reset`))))))))

(fn `UserConstructionScript`)