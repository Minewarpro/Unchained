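; BP_LightFour is a point light, apparently for an oven or furnace ("four"), that switches on and off by reference count.
; LightUp and Lightdown adjust an active counter, playing an intensity timeline on the first activation and reversing it faster when the count returns to zero.
; The construction script applies the initial intensity.
; A self-retriggering random flicker event, Clignotement, exists, but nothing in this Blueprint starts it.
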(event `self.ReceiveBeginPlay`)

(event `Clignotement`
  (bind _returnvalue (`KismetMathLibrary.RandomFloatInRange` 0.3 0.5))
  (`KismetSystemLibrary.Delay` _returnvalue)
  (`TimelineComponent.SetPlayRate` (`self.TimelineClignotement`) (/ 1.0 _returnvalue))
  (bind (_direction _newtrack_0) (`Timeline|TimelineClignotement` :!via `PlayFromStart`)
    (:`Update`
      (bind _returnvalue_2 (`KismetMathLibrary.Lerp` (`self.intensity temp`) (`KismetMathLibrary.RandomFloatInRange` 15.0 35.0) _newtrack_0))
      (set `self.intensity temp` _returnvalue_2)
      (`LightComponent.SetIntensity` (`self.PointLight`) _returnvalue_2)
      (`self.Clignotement`))))

(event `Light Up`
  (bind _output_get (set `self.nb four active light` (+ (`self.nb four active light`) 1)))
  (if (== _output_get 1)
    (`TimelineComponent.SetPlayRate` (`self.Light Intensity Timeline`) 1.0)
    (bind (_direction _newtrack_0) (`Timeline|Light Intensity Timeline` :!label _label)
      (:`Update`
        (`LightComponent.SetIntensity` (`self.PointLight`) (* _newtrack_0 10.0))))))

(event `Light down`
  (bind _output_get (set `self.nb four active light` (- (`self.nb four active light`) 1)))
  (if (== _output_get 0)
    (`TimelineComponent.SetPlayRate` (`self.Light intensity timeline`) 2.0)
    (goto _label :!via `Reverse`)))

(fn `UserConstructionScript`
  (bind _intensity (`self.Intensity`))
  (`LightComponent.SetIntensity` (`self.PointLight`) _intensity)
  (set `self.intensity temp` _intensity))