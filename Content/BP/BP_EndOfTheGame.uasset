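; BP_EndOfTheGame is a trigger box that plays the ending sequence once when BP_Player overlaps it, then returns to the main menu.
; It creates a WB_EndGame widget and uses timelines to fade in a white screen, disable input, then fade in and slide the title text.
; After a pause it reverses a third timeline to fade the text out and opens MainMenuMap, with fade speeds derived from configurable durations.
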(event `self.Box.OnComponentBeginOverlap`
  (params (OverlappedComponent :type "PrimitiveComponent Object Reference") (OtherActor :type "Actor Object Reference") (OtherComp :type "PrimitiveComponent Object Reference") (OtherBodyIndex :type Integer) (bFromSweep :type Boolean) (SweepResult :type "HitResult Structure (by ref)"))
  (bind _wb_end_ref (`self.WB End Ref`))
  (cast `/Game/BP/BP_Player` OtherActor)
  (`/Engine/EditorBlueprintResources/StandardMacros.DoOnce` false
    (:`Completed`
      (bind _returnvalue (`|CreateWidget` "/Game/BP/ui/WB_EndGame.WB_EndGame_C"))
      (bind _output_get (set `self.WB End Ref` _returnvalue))
      (`UserWidget.AddToViewport` _returnvalue 0)
      (`UserWidget.AddToViewport` _output_get 0)
      (`TimelineComponent.SetPlayRate` (`self.WhiteApparition`) (/ 1.0 (`self.time apparition in s`)))
      (bind (_direction _opacity) (`Timeline|WhiteApparition`)
        (:`Update`
          (set `/Game/BP/ui/WB_EndGame.WhiteOpacity` _opacity (`self.WB End Ref`)))
        (:`Finished`
          (`self.DisableInput` (`GameplayStatics.GetPlayerController` 0))
          (`KismetSystemLibrary.Delay` 2.0)
          (`TimelineComponent.SetPlayRate` (`self.TextApparition`) (/ 1.0 (`self.Time apparition text in s`)))
          (bind (_direction_2 _opacity_2 _ylocation) (`Timeline|TextApparition`)
            (:`Update`
              (set `/Game/BP/ui/WB_EndGame.TextOpacity` _opacity_2 _wb_end_ref)
              (set `Widget.RenderTransform` (make `WidgetTransform` (`KismetMathLibrary.MakeVector2D` 0.0 (* _ylocation -30.0))) (`/Game/BP/ui/WB_EndGame.Text_Title` _wb_end_ref)))
            (:`Finished`
              (`KismetSystemLibrary.Delay` 5.0)
              (`TimelineComponent.SetPlayRate` (`self.TextDisparrition`) (/ 1.0 (`self.Time apparition text in s`)))
              (bind (_direction_3 _opacity_3) (`Timeline|TextDisparrition` :!via `ReverseFromEnd`)
                (:`Update`
                  (set `/Game/BP/ui/WB_EndGame.TextOpacity` _opacity_3 (`self.WB End Ref`)))
                (:`Finished`
                  (`GameplayStatics.OpenLevel` "MainMenuMap"))))))))))

(fn `UserConstructionScript`)