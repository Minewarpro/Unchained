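; Gameplay-brick Blueprint for a beam extremity ("PoutreFour") that moves and rotates its static mesh to a target transform when activated.
; ActivateObject captures the mesh's starting world rotation and, through a DoOnce, plays the Deplacement timeline a single time.
; The timeline's per-axis Location and Rotation curves interpolate from InitWorldLocation and InitWorldRotation to LocationTo and RotationTo in world space.
; InitWorldLocation is never assigned in this graph.
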(event `/Game/BP/Briques_De_Jeu/BPI_ActivateObject.ActivateObject`
  (bind (_locationto_x _locationto_y _locationto_z) (`KismetMathLibrary.BreakVector` (`self.LocationTo`)))
  (bind (_initworldlocation_x _initworldlocation_y _initworldlocation_z) (`KismetMathLibrary.BreakVector` (`self.InitWorldLocation`)))
  (bind (_initworldlocation_x_2 _initworldlocation_y_2 _initworldlocation_z_2) (`KismetMathLibrary.BreakVector` (`self.InitWorldLocation`)))
  (bind (_rotationto_roll _rotationto_pitch _rotationto_yaw) (`KismetMathLibrary.BreakRotator` (`self.RotationTo`)))
  (bind (_initworldrotation_roll _initworldrotation_pitch _initworldrotation_yaw) (`KismetMathLibrary.BreakRotator` (`self.InitWorldRotation`)))
  (bind (_initworldrotation_roll_2 _initworldrotation_pitch_2 _initworldrotation_yaw_2) (`KismetMathLibrary.BreakRotator` (`self.InitWorldRotation`)))
  (set `self.InitWorldRotation` (`SceneComponent.K2_GetComponentRotation` (`self.StaticMesh`)))
  (`/Engine/EditorBlueprintResources/StandardMacros.DoOnce` false
    (:`Completed`
      (bind (_direction _rotation _location) (`Timeline|Deplacement` :!via `PlayFromStart`)
        (:`Update`
          (`SceneComponent.K2_SetWorldLocationAndRotation` (`self.StaticMesh`) (`KismetMathLibrary.MakeVector` (+ (* (.x _location) (- _locationto_x _initworldlocation_x_2)) _initworldlocation_x) (+ (* (.y _location) (- _locationto_y _initworldlocation_y_2)) _initworldlocation_y) (+ (* (.z _location) (- _locationto_z _initworldlocation_z_2)) _initworldlocation_z)) (`KismetMathLibrary.MakeRotator` (+ (* (.x _rotation) (- _rotationto_roll _initworldrotation_roll)) _initworldrotation_roll_2) (+ (* (.y _rotation) (- _rotationto_pitch _initworldrotation_pitch)) _initworldrotation_pitch_2) (+ (* (.z _rotation) (- _rotationto_yaw _initworldrotation_yaw)) _initworldrotation_yaw_2)) false false))))))

(fn `UserConstructionScript`)