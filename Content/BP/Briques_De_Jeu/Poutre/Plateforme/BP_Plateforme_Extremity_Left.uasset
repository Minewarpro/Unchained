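; Left-extremity platform piece that rotates its static mesh to a target rotation once it has received the required number of activation calls.
; A one-shot gate starts a timeline that blends each axis from the initial world rotation, with mesh collision disabled during the move.
; When finished, collision returns and a player overlapping the box is repeatedly impulsed backward along the capsule's forward axis, after short delays, until clear.
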(event `/Game/BP/Briques_De_Jeu/BPI_ActivateObject.ActivateObject`
  (bind (_rotationto_roll _rotationto_pitch _rotationto_yaw) (`KismetMathLibrary.BreakRotator` (`self.RotationTo`)))
  (bind (_initworldrotation_roll _initworldrotation_pitch _initworldrotation_yaw) (`KismetMathLibrary.BreakRotator` (`self.InitWorldRotation`)))
  (bind (_initworldrotation_roll_2 _initworldrotation_pitch_2 _initworldrotation_yaw_2) (`KismetMathLibrary.BreakRotator` (`self.InitWorldRotation`)))
  (bind _output_get (set `self.nb temp` (+ (`self.nb temp`) 1)))
  (if (== _output_get (`self.nb to activate`))
    (set `self.InitWorldRotation` (`SceneComponent.K2_GetComponentRotation` (`self.StaticMesh`)))
    (`/Engine/EditorBlueprintResources/StandardMacros.DoOnce` false
      (:`Completed`
        (`PrimitiveComponent.SetCollisionEnabled` (`self.StaticMesh`) "NoCollision")
        (bind (_direction _rotation) (`Timeline|Deplacement` :!via `PlayFromStart`)
          (:`Update`
            (`SceneComponent.K2_SetWorldRotation` (`self.StaticMesh`) (`KismetMathLibrary.MakeRotator` (+ (* (.x _rotation) (- _rotationto_roll _initworldrotation_roll)) _initworldrotation_roll_2) (+ (* (.y _rotation) (- _rotationto_pitch _initworldrotation_pitch)) _initworldrotation_pitch_2) (+ (* (.z _rotation) (- _rotationto_yaw _initworldrotation_yaw)) _initworldrotation_yaw_2)) false false))
          (:`Finished`
            (`PrimitiveComponent.SetCollisionEnabled` (`self.StaticMesh`) "QueryAndPhysics")
            (`self.Pousse`)))))))

(event `Pousse`
  (`KismetSystemLibrary.Delay` 0.1)
  (bind _asbp_player (cast `/Game/BP/BP_Player` (`GameplayStatics.GetPlayerPawn` 0)))
  (bind _capsule (`/Game/BP/BP_Player.Capsule` _asbp_player))
  (if (`PrimitiveComponent.IsOverlappingComponent` (`self.Box`) _capsule)
    (`PrimitiveComponent.AddVelocityChangeImpulseAtLocation` _capsule (* (`SceneComponent.GetForwardVector` _capsule) -1000.0) (`SceneComponent.K2_GetComponentLocation` _capsule) "None")
    (`self.Pousse`)))

(fn `UserConstructionScript`)