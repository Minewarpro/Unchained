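; BP_PoutreFour_Extremity_Rotation is a beam-extremity gameplay brick that rotates its static mesh to a target orientation when activated.
; ActivateObject stores the mesh's current world rotation, then a DoOnce starts the Deplacement timeline.
; Each update interpolates roll, pitch and yaw separately toward RotationTo, weighted by the timeline's vector track.
; On finish, it prints the resulting rotation.
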(event `/Game/BP/Briques_De_Jeu/BPI_ActivateObject.ActivateObject`
  (bind (_rotationto_roll _rotationto_pitch _rotationto_yaw) (`KismetMathLibrary.BreakRotator` (`self.RotationTo`)))
  (bind (_initworldrotation_roll _initworldrotation_pitch _initworldrotation_yaw) (`KismetMathLibrary.BreakRotator` (`self.InitWorldRotation`)))
  (bind (_initworldrotation_roll_2 _initworldrotation_pitch_2 _initworldrotation_yaw_2) (`KismetMathLibrary.BreakRotator` (`self.InitWorldRotation`)))
  (set `self.InitWorldRotation` (`SceneComponent.K2_GetComponentRotation` (`self.StaticMesh`)))
  (`/Engine/EditorBlueprintResources/StandardMacros.DoOnce` false
    (:`Completed`
      (bind (_direction _rotation) (`Timeline|Deplacement` :!via `PlayFromStart`)
        (:`Update`
          (`SceneComponent.K2_SetWorldRotation` (`self.StaticMesh`) (`KismetMathLibrary.MakeRotator` (+ (* (.x _rotation) (- _rotationto_roll _initworldrotation_roll)) _initworldrotation_roll_2) (+ (* (.y _rotation) (- _rotationto_pitch _initworldrotation_pitch)) _initworldrotation_pitch_2) (+ (* (.z _rotation) (- _rotationto_yaw _initworldrotation_yaw)) _initworldrotation_yaw_2)) false false))
        (:`Finished`
          (`KismetSystemLibrary.PrintString` (`KismetStringLibrary.Conv_RotatorToString` (`SceneComponent.K2_GetComponentRotation` (`self.StaticMesh`)))))))))

(fn `UserConstructionScript`)