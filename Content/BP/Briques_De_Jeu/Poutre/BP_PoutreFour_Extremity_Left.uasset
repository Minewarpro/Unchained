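; Left end piece of the "PoutreFour" beam gameplay brick, which rotates its static mesh once enough activations have been received.
; ActivateObject counts calls and, when the count equals NbToActivate, captures the current world rotation and passes a DoOnce gate to play the Deplacement timeline.
; The timeline's Rotation vector curve interpolates roll, pitch and yaw independently from that captured rotation to the absolute RotationTo target.
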(event `/Game/BP/Briques_De_Jeu/BPI_ActivateObject.ActivateObject`
  (bind (_rotationto_roll _rotationto_pitch _rotationto_yaw) (`KismetMathLibrary.BreakRotator` (`self.RotationTo`)))
  (bind (_initworldrotation_roll _initworldrotation_pitch _initworldrotation_yaw) (`KismetMathLibrary.BreakRotator` (`self.InitWorldRotation`)))
  (bind (_initworldrotation_roll_2 _initworldrotation_pitch_2 _initworldrotation_yaw_2) (`KismetMathLibrary.BreakRotator` (`self.InitWorldRotation`)))
  (bind _output_get (set `self.nb temp` (+ (`self.nb temp`) 1)))
  (if (== _output_get (`self.nb to activate`))
    (set `self.InitWorldRotation` (`SceneComponent.K2_GetComponentRotation` (`self.StaticMesh`)))
    (`/Engine/EditorBlueprintResources/StandardMacros.DoOnce` false
      (:`Completed`
        (bind (_direction _rotation) (`Timeline|Deplacement` :!via `PlayFromStart`)
          (:`Update`
            (`SceneComponent.K2_SetWorldRotation` (`self.StaticMesh`) (`KismetMathLibrary.MakeRotator` (+ (* (.x _rotation) (- _rotationto_roll _initworldrotation_roll)) _initworldrotation_roll_2) (+ (* (.y _rotation) (- _rotationto_pitch _initworldrotation_pitch)) _initworldrotation_pitch_2) (+ (* (.z _rotation) (- _rotationto_yaw _initworldrotation_yaw)) _initworldrotation_yaw_2)) false false)))))))

(fn `UserConstructionScript`)