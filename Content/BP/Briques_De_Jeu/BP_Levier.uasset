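; BP_Levier is a physics lever gameplay brick that activates a linked BP_CrochetVertical when the player's rope overlaps its box.
; The first rope overlap releases the "bouge" constraint's angular drive and notifies the hook, gated by a DoOnce.
; ResetLevier restores the drive's spring strength and re-arms that gate.
; Tick pitches BoxPivot from the simulated lever's socket roll, keeping the box aligned with its motion.
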(event `self.ReceiveTick`
  (params (DeltaSeconds :type "Float (single-precision)"))
  (bind _returnvalue_roll (`KismetMathLibrary.BreakRotator` (`SceneComponent.GetSocketRotation` (`self.Levier__2_`) "bougeSocket")))
  (`SceneComponent.K2_SetRelativeRotation` (`self.BoxPivot`) (`KismetMathLibrary.MakeRotator` 0.0 (- _returnvalue_roll 50.0)) false false))

(event `ResetLevier`
  (bind _levier__2_ (`self.Levier__2_`))
  (`KismetSystemLibrary.PrintString` "rset levier")
  (bind _returnvalue (`SkeletalMeshComponent.GetConstraintByName` _levier__2_ "bouge" false))
  (`ConstraintInstanceBlueprintLibrary.SetAngularDriveParams` _returnvalue 10.0 0.0)
  (`PrimitiveComponent.SetSimulatePhysics` _levier__2_ true)
  (goto _label :!via `Reset`))

(event `self.Box.OnComponentBeginOverlap`
  (params (OverlappedComponent :type "PrimitiveComponent Object Reference") (OtherActor :type "Actor Object Reference") (OtherComp :type "PrimitiveComponent Object Reference") (OtherBodyIndex :type Integer) (bFromSweep :type Boolean) (SweepResult :type "HitResult Structure (by ref)"))
  (bind _asbp_player (cast `/Game/BP/BP_Player` OtherActor))
  (if (== (`/Game/BP/BP_Player.Rope` _asbp_player) OtherComp)
    (set `self.Chain on ` true)
    (`KismetSystemLibrary.PrintString` "overlap levier")
    (`/Engine/EditorBlueprintResources/StandardMacros.DoOnce` false :!label _label
      (:`Completed`
        (bind _returnvalue (`SkeletalMeshComponent.GetConstraintByName` (`self.Levier__2_`) "bouge" false))
        (`ConstraintInstanceBlueprintLibrary.SetAngularDriveParams` _returnvalue 0.0)
        (`PrimitiveComponent.SetSimulatePhysics` (`self.Levier__2_`) true)
        (bind _asbp_crochet_vertical (cast `/Game/BP/Briques_De_Jeu/BP_CrochetVertical` (`self.Object To Activate`)))
        (`/Game/BP/Briques_De_Jeu/BP_CrochetVertical.ActiveByLever` _asbp_crochet_vertical self)))))

(event `self.Box.OnComponentEndOverlap`
  (params (OverlappedComponent :type "PrimitiveComponent Object Reference") (OtherActor :type "Actor Object Reference") (OtherComp :type "PrimitiveComponent Object Reference") (OtherBodyIndex :type Integer))
  (bind _asbp_player (cast `/Game/BP/BP_Player` OtherActor))
  (if (== (`/Game/BP/BP_Player.Rope` _asbp_player) OtherComp)
    (set `self.Chain on ` false)
    (`KismetSystemLibrary.PrintString` "overlap end levier")))

(fn `UserConstructionScript`)