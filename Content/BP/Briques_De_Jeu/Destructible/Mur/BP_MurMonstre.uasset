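; BP_MurMonstre is a destructible wall variant that brings the monster to its location when activated.
; It caches the BP_NPC monster and its AI_NPC on BeginPlay.
; ActivateObject teleports the monster to the SpawnMOnstre component's transform, makes the AI scream, activates a Niagara effect, then destroys the wall.
; A BP_Mur spawn step is left unconnected and never runs.
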(event `self.ReceiveBeginPlay`
  (bind _returnvalue (`GameplayStatics.GetActorOfClass` "/Game/Characters/AI/BP_NPC.BP_NPC_C"))
  (set `self.Monster` _returnvalue)
  (bind _returnvalue_2 (`GameplayStatics.GetActorOfClass` "/Game/Characters/AI/AI_NPC.AI_NPC_C"))
  (set `self.AI` _returnvalue_2))

(event `/Game/BP/Briques_De_Jeu/BPI_ActivateObject.ActivateObject`
  (bind _spawn_monstre (`self.Spawn MOnstre`))
  (`self.K2_SetActorLocationAndRotation` (`self.Monster`) (`SceneComponent.K2_GetComponentLocation` _spawn_monstre) (`SceneComponent.K2_GetComponentRotation` _spawn_monstre) false true)
  (`/Game/Characters/AI/AI_NPC.Scream` (`self.AI`))
  (`ActorComponent.Activate` (`self.Niagara`) false)
  (`self.K2_DestroyActor`))

(fn `UserConstructionScript`)