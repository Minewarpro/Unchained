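; BP_Mur is a destructible wall that also relocates the monster when the player comes near.
; It finds the BP_NPC at BeginPlay and teleports it to the Box component's location whenever the player pawn overlaps the Sphere, whether or not the wall is broken.
; On a Chaos break, the destructible components ignore a custom collision channel.
; The construction script draws a debug sphere at the trigger's location.
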(event `self.ReceiveBeginPlay`
  (bind _returnvalue (`GameplayStatics.GetActorOfClass` "/Game/Characters/AI/BP_NPC.BP_NPC_C"))
  (set `self.MonsterRef` _returnvalue))

(event `self.DestructibleObject.OnChaosBreakEvent`
  (params (BreakEvent :type "ChaosBreakEvent Structure (by ref)"))
  (`PrimitiveComponent.SetCollisionResponseToChannel` (`self.DestructibleObject`) "ECC_GameTraceChannel3" "ECR_Ignore")
  (`PrimitiveComponent.SetCollisionResponseToChannel` (`self.GeometryCollectionComponent`) "ECC_GameTraceChannel3" "ECR_Ignore"))

(event `self.Sphere.OnComponentBeginOverlap`
  (params (OverlappedComponent :type "PrimitiveComponent Object Reference") (OtherActor :type "Actor Object Reference") (OtherComp :type "PrimitiveComponent Object Reference") (OtherBodyIndex :type Integer) (bFromSweep :type Boolean) (SweepResult :type "HitResult Structure (by ref)"))
  (if (== OtherActor (`GameplayStatics.GetPlayerPawn` 0))
    (`self.K2_SetActorLocation` (`self.MonsterRef`) (`SceneComponent.K2_GetComponentLocation` (`self.Box`)) false true)))

(fn `UserConstructionScript`
  (`KismetSystemLibrary.DrawDebugSphere` (`SceneComponent.K2_GetComponentLocation` (`self.Sphere`)) 300.0))