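; BP_Balancoire is a seesaw or swing gameplay brick that, as wired, acts as a launcher for BP_Player.
; It caches the player on BeginPlay, and the A key applies a large forward (+X) and upward force to the player's Capsule.
; A timeline that tilts the Cube and a smaller push on the player's Boulet are left disconnected, so the brick itself never moves.
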(event `self.ReceiveBeginPlay`
  (bind _returnvalue (`GameplayStatics.GetActorOfClass` "/Game/BP/BP_Player.BP_Player_C"))
  (set `self.NewVar` _returnvalue))

(event `Key|A`
  (params (Key :type "Key Structure"))
  (:`Pressed`
    (`PrimitiveComponent.AddForce` (`/Game/BP/BP_Player.Capsule` (`self.NewVar`)) (110000000.0 0.0 600000000.0) "None" false)))

(fn `UserConstructionScript`)