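; Sliding beam level brick that acts as a zipline for BP_Player's rope.
; When the rope overlaps the resizable Box, it lightens the player's Mass and passes itself to the player; on exit it restores a heavy Mass, clears OnZipline and stops the sound.
; Playsound, not called within this Blueprint, starts the audio and a looping timer that keeps it at the player's Boulet position.
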(event `Sound On Boulet`
  (`SceneComponent.K2_SetWorldLocation` (`self.AudioCurveSource`) (`SceneComponent.K2_GetComponentLocation` (`/Game/BP/BP_Player.Boulet` (`self.As BP Player`))) false false))

(event `Play sound`
  (`AudioComponent.Play` (`self.AudioCurveSource`) 0.0)
  (bind _returnvalue (`KismetSystemLibrary.K2_SetTimerDelegate` (delegate `Sound On Boulet`) 0.05 true))
  (set `self.Timer Boulet Location` _returnvalue)
  (`self.Sound On Boulet`))

(event `Stop Sound`
  (`AudioComponent.Stop` (`self.AudioCurveSource`))
  (`KismetSystemLibrary.K2_ClearAndInvalidateTimerHandle` (`self.Timer Boulet Location`)))

(event `self.Box.OnComponentBeginOverlap`
  (params (OverlappedComponent :type "PrimitiveComponent Object Reference") (OtherActor :type "Actor Object Reference") (OtherComp :type "PrimitiveComponent Object Reference") (OtherBodyIndex :type Integer) (bFromSweep :type Boolean) (SweepResult :type "HitResult Structure (by ref)"))
  (bind _asbp_player (cast `/Game/BP/BP_Player` OtherActor))
  (set `self.As BP Player` _asbp_player)
  (if (== (`/Game/BP/BP_Player.Rope` _asbp_player) OtherComp)
    (set `/Game/BP/BP_Player.Mass` 1.0 _asbp_player)
    (`/Game/BP/BP_Player.Receive Info Zipline` _asbp_player self)))

(event `self.Box.OnComponentEndOverlap`
  (params (OverlappedComponent :type "PrimitiveComponent Object Reference") (OtherActor :type "Actor Object Reference") (OtherComp :type "PrimitiveComponent Object Reference") (OtherBodyIndex :type Integer))
  (bind _asbp_player (cast `/Game/BP/BP_Player` OtherActor))
  (if (== (`/Game/BP/BP_Player.Rope` _asbp_player) OtherComp)
    (set `/Game/BP/BP_Player.Mass` 500.0 _asbp_player)
    (`self.Stop Sound`)
    (set `/Game/BP/BP_Player.OnZipline` false _asbp_player)))

(fn `UserConstructionScript`
  (`BoxComponent.SetBoxExtent` (`self.Box`) (`self.In Box Extent`) true))