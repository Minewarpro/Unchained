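; BP_TirageCrochet_Chaudron is a hook-pull gameplay brick that progressively opens a cauldron as its physics Cube moves away from its Soutien (support).
; On Tick, while the Cube moves, it measures the offset Cube-to-support distance and passes it, normalized, to OpeningChaudron on the BP_ChaudronTiming in ObjectToActivate.
; Near full extension it instead disables the Cube's physics simulation, locking the pull.
; BeginPlay caches a player reference that the graph never uses.
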(event `self.ReceiveBeginPlay`
  (`self.Get Relative Location`)
  (bind _returnvalue (`GameplayStatics.GetActorOfClass` "/Game/BP/BP_Player.BP_Player_C"))
  (set `self.PlayerRef` _returnvalue))

(event `self.ReceiveTick`
  (params (DeltaSeconds :type "Float (single-precision)"))
  (bind (_returnvalue_x _returnvalue_y _returnvalue_z) (`KismetMathLibrary.BreakVector` (`SceneComponent.GetComponentVelocity` (`self.Cube`))))
  (if (or (!= _returnvalue_x 0.0) (!= _returnvalue_y 0.0) (!= _returnvalue_z 0.0))
    (bind _relative_distance (`self.Get Relative Location`))
    (if (>= _relative_distance 195.0)
      (`PrimitiveComponent.SetSimulatePhysics` (`self.Cube`) false)
      (else
        (bind _asbp_chaudron_timing (cast `/Game/BP/Briques_De_Jeu/BP_ChaudronTiming` (`self.Object to activate`)))
        (`/Game/BP/Briques_De_Jeu/BP_ChaudronTiming.OpeningChaudron` _asbp_chaudron_timing (`KismetMathLibrary.Abs` (`KismetMathLibrary.NormalizeToRange` _relative_distance 0.0 200.0)))))))

(fn `Get Relative Location`
  (returns (`relative distance` :type "Float (double-precision)"))
  (bind _output_get (set `self.Relative Distance Cube` (- (`KismetMathLibrary.Vector_Distance` (`SceneComponent.K2_GetComponentLocation` (`self.Cube`)) (`SceneComponent.K2_GetComponentLocation` (`self.Soutien`))) 255.0)))
  (return _output_get))

(fn `UserConstructionScript`)