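; BP_TirageCrochet is a gameplay brick, apparently a hook pull, whose moving cube drives a BP_DoorTiming door.
; Each tick it checks whether the cube's velocity is positive on any axis, so purely negative motion is ignored.
; While it is, it casts ObjectToActivate to BP_DoorTiming and calls Opening with the cube's relative X location scaled down to an opening ratio.
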(event `self.ReceiveTick`
  (params (DeltaSeconds :type "Float (single-precision)"))
  (bind (_returnvalue_x _returnvalue_y _returnvalue_z) (`KismetMathLibrary.BreakVector` (`SceneComponent.GetComponentVelocity` (`self.Cube`))))
  (bind _relativelocation_x (`KismetMathLibrary.BreakVector` (`SceneComponent.RelativeLocation` (`self.Cube`))))
  (if (or (> _returnvalue_x 0.0) (> _returnvalue_y 0.0) (> _returnvalue_z 0.0))
    (bind _asbp_door_timing (cast `/Game/BP/Briques_De_Jeu/BP_DoorTiming` (`self.Object to activate`)))
    (`/Game/BP/Briques_De_Jeu/BP_DoorTiming.Opening` _asbp_door_timing (/ _relativelocation_x 200.0))))

(fn `UserConstructionScript`)