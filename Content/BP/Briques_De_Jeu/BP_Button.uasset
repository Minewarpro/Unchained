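; BP_Button is a pressure button that activates a linked object through interface-style messages when components overlap its box.
; A press needs more than one overlapping component, plays a sound, moves the cylinder by timeline and can trigger a second object once.
; With ReverseButton set, an empty box deactivates the object and reverses the timeline.
; Two DoOnce gates reset each other so press and release alternate.
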(event `/Game/BP/Briques_De_Jeu/BPI_Interacts.Interacts`
  (`/Engine/EditorBlueprintResources/StandardMacros.DoOnce` false :!label _label
    (:`Completed`
      (message `/Game/BP/Briques_De_Jeu/BPI_ActivateObject.ActivateObject` (`self.ObjectToActivate`))
      (`GameplayStatics.PlaySoundAtLocation` "/Game/SFX/Environnement/Cue_ButtonPress.Cue_ButtonPress" (`self.K2_GetActorLocation`) (struct) 1.0 1.0 0.0 null null null null)
      (bind (_direction _move) (`Timeline|Timeline` :!label _label_2)
        (:`Update`
          (`SceneComponent.K2_SetRelativeLocation` (`self.Cylinder`) (`KismetMathLibrary.MakeVector` 0.0 0.0 (* _move 100.0)) false false))))))

(event `self.Box.OnComponentEndOverlap`
  (params (OverlappedComponent :type "PrimitiveComponent Object Reference") (OtherActor :type "Actor Object Reference") (OtherComp :type "PrimitiveComponent Object Reference") (OtherBodyIndex :type Integer))
  (if (`self.ReverseButton`)
    (if (== (`KismetArrayLibrary.Array_Length` (`PrimitiveComponent.GetOverlappingComponents` (`self.Box`))) 0)
      (`|ExecutionSequence`
        (:`then_0`
          (goto _label :!via `Reset`))
        (:`then_1`
          (`/Engine/EditorBlueprintResources/StandardMacros.DoOnce` false :!label _label_3
            (:`Completed`
              (message `/Game/BP/Briques_De_Jeu/BPI_DesactivateObject.DesactivateObject` (`self.ObjectToActivate`))
              (`GameplayStatics.PlaySoundAtLocation` "/Game/SFX/Environnement/Cue_ButtonUp.Cue_ButtonUp" (`self.K2_GetActorLocation`) (struct) 1.0 1.0 0.0 null null null null)
              (goto _label_2 :!via `Reverse`))))))))

(event `self.Box.OnComponentBeginOverlap`
  (params (OverlappedComponent :type "PrimitiveComponent Object Reference") (OtherActor :type "Actor Object Reference") (OtherComp :type "PrimitiveComponent Object Reference") (OtherBodyIndex :type Integer) (bFromSweep :type Boolean) (SweepResult :type "HitResult Structure (by ref)"))
  (if (> (`KismetArrayLibrary.Array_Length` (`PrimitiveComponent.GetOverlappingComponents` (`self.Box`))) 1)
    (`/Game/BP/Briques_De_Jeu/BPI_Interacts.Interacts`)
    (`|ExecutionSequence`
      (:`then_0`
        (goto _label_3 :!via `Reset`))
      (:`then_1`
        (if (`self.need Activate other event`)
          (`/Engine/EditorBlueprintResources/StandardMacros.DoOnce` false
            (:`Completed`
              (message `/Game/BP/Briques_De_Jeu/BPI_ActivateObject.ActivateObject` (`self.other event`)))))))))

(fn `UserConstructionScript`)