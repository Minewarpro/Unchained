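; BP_Doors is a lockable door that swings open and closed on interaction, with a point light showing its lock state.
; Construction colors the light red when CanOpen is false; ActivateObject turns it green, unlocks the door and immediately runs the same toggle as Interacts.
; If CanOpen is true, a FlipFlop alternately plays and reverses the Open timeline, which drives the Porte yaw up to a quarter turn.
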(event `/Game/BP/Briques_De_Jeu/BPI_ActivateObject.ActivateObject`
  (`LightComponent.SetLightColor` (`self.PointLight`) (make `LinearColor` 0.0 1.0 0.0 1.0) true)
  (set `self.CanOpen` true)
  (if (`self.CanOpen`) :!label _label
    (`/Engine/EditorBlueprintResources/StandardMacros.FlipFlop`
      (:`A`
        (bind (_direction _z_rotate) (`Timeline|Open` :!label _label_2)
          (:`Update`
            (`SceneComponent.K2_SetRelativeRotation` (`self.Porte`) (`KismetMathLibrary.MakeRotator` 0.0 0.0 (* _z_rotate 90.0)) false false))))
      (:`B`
        (goto _label_2 :!via `Reverse`)))))

(event `/Game/BP/Briques_De_Jeu/BPI_Interacts.Interacts`
  (goto _label))

(fn `UserConstructionScript`
  (if (not (`self.CanOpen`))
    (`LightComponent.SetLightColor` (`self.PointLight`) (make `LinearColor` 1.0 0.0 0.0 1.0) true)))