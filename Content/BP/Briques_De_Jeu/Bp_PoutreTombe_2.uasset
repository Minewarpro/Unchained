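; Breakable beam gameplay brick that topples once when the player's thrown Boulet hits it.
; The Box overlap checks that the overlapping component is the player's Boulet and that it is being thrown.
; The hit destroys two plank meshes, triggers a Niagara effect and break sound, and calls Tombe.
; Tombe plays a half-speed timeline that pitches the beam's pivot up to 90 degrees, scaled by the curve.
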(event `Tombe`
  (`TimelineComponent.SetPlayRate` (`self.TombeTimelin`) (/ 1.0 2.0))
  (bind (_direction _y_rotation) (`Timeline|TombeTimelin` :!via `PlayFromStart`)
    (:`Update`
      (`SceneComponent.K2_SetRelativeRotation` (`self.poutrepivot`) (`KismetMathLibrary.MakeRotator` 0.0 (* _y_rotation 90.0)) false false))))

(event `self.Box.OnComponentBeginOverlap`
  (params (OverlappedComponent :type "PrimitiveComponent Object Reference") (OtherActor :type "Actor Object Reference") (OtherComp :type "PrimitiveComponent Object Reference") (OtherBodyIndex :type Integer) (bFromSweep :type Boolean) (SweepResult :type "HitResult Structure (by ref)"))
  (bind _asbp_player (cast `/Game/BP/BP_Player` OtherActor))
  (if (== (`/Game/BP/BP_Player.Boulet` _asbp_player) OtherComp)
    (if (`/Game/BP/BP_Player.throwing boulet` _asbp_player)
      (`/Engine/EditorBlueprintResources/StandardMacros.DoOnce` false
        (:`Completed`
          (`self.Tombe`)
          (`ActorComponent.Activate` (`self.NS_PlancheDestroy`) false)
          (`ActorComponent.K2_DestroyComponent` (`self.Planche_Low2`))
          (`ActorComponent.K2_DestroyComponent` (`self.Planche_Low1`))
          (`GameplayStatics.PlaySoundAtLocation` "/Game/SFX/Environnement/CaisseBreak.CaisseBreak" (`self.K2_GetActorLocation`) (struct) 1.0 1.0 0.0 null null null null))))))

(fn `UserConstructionScript`)