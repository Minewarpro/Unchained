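; Zipline path actor that spawns BP_Tirolienne hooks on a looping timer and sends them travelling along its spline.
; The construction script places a machine mesh at a normalized distance along the spline, with an offset trigger box beside it.
; The first player overlap with that box calls StopCollide on the zipline hook stored in TyroRef, which is assigned through the GetTyroRef event.
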(event `self.ReceiveBeginPlay`
  (`KismetSystemLibrary.K2_SetTimerDelegate` (delegate `Spawn Crochet`) (`self.Delay to spawn in s`) true)
  (`self.Spawn Crochet`))

(event `Spawn Crochet`
  (bind _returnvalue (`|SpawnActorFromClass` "/Game/BP/Briques_De_Jeu/BP_Tirolienne.BP_Tirolienne_C" (`KismetMathLibrary.MakeTransform` (`SceneComponent.K2_GetComponentLocation` (`self.Spline`))) "Undefined" "OverrideRootScale" null null))
  (`/Game/BP/Briques_De_Jeu/BP_Tirolienne.Move` _returnvalue (`self.Spline`) (`self.Time to Travel`) self))

(event `self.Box.OnComponentBeginOverlap`
  (params (OverlappedComponent :type "PrimitiveComponent Object Reference") (OtherActor :type "Actor Object Reference") (OtherComp :type "PrimitiveComponent Object Reference") (OtherBodyIndex :type Integer) (bFromSweep :type Boolean) (SweepResult :type "HitResult Structure (by ref)"))
  (cast `/Game/BP/BP_Player` OtherActor)
  (`/Engine/EditorBlueprintResources/StandardMacros.DoOnce` false
    (:`Completed`
      (bind _asbp_tirolienne (cast `/Game/BP/Briques_De_Jeu/BP_Tirolienne` (`self.Tyro Ref`)))
      (`/Game/BP/Briques_De_Jeu/BP_Tirolienne.StopCollide` _asbp_tirolienne))))

(event `GetTyroRef`
  (params (TyroRef :type "Actor Object Reference"))
  (set `self.Tyro Ref` TyroRef))

(fn `UserConstructionScript`
  (bind _spline (`self.Spline`))
  (bind _returnvalue (`KismetMathLibrary.Lerp` 0.0 (`SplineComponent.GetSplineLength` _spline) (`self.DistanceSpline`)))
  (bind (_returnvalue_roll _returnvalue_pitch _returnvalue_yaw) (`KismetMathLibrary.BreakRotator` (`SplineComponent.GetRotationAtDistanceAlongSpline` _spline _returnvalue "Local")))
  (bind (_returnvalue_x _returnvalue_y _returnvalue_z) (`KismetMathLibrary.BreakVector` (`SplineComponent.GetLocationAtDistanceAlongSpline` _spline _returnvalue "Local")))
  (bind _returnvalue_2 (`AddComponent|NODE_AddStaticMeshComponent-0` :`RelativeTransform` (`KismetMathLibrary.MakeTransform` (`KismetMathLibrary.MakeVector` _returnvalue_x _returnvalue_y (+ _returnvalue_z (`self.hauteur`))) (`KismetMathLibrary.MakeRotator` (+ _returnvalue_roll 180.0) _returnvalue_pitch (+ _returnvalue_yaw -90.0)) (`KismetMathLibrary.Conv_DoubleToVector` (`self.MachineScale`)))))
  (bind _returnvalue_3 (`SceneComponent.GetRelativeTransform` _returnvalue_2))
  (bind _returnvalue_4 (`AddComponent|NODE_AddBoxComponent-0` :`RelativeTransform` (`KismetMathLibrary.MakeTransform` (`KismetMathLibrary.MakeVector` (+ (.x (.location _returnvalue_3)) (`self.XOffset`)) (.y (.location _returnvalue_3)) (+ (.z (.location _returnvalue_3)) (`self.ZOffset`))) (.rotation _returnvalue_3) (`self.ScaleBox`))))
  (set `self.Box` _returnvalue_4))