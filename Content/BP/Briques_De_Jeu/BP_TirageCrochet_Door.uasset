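; Hook-pull door mechanism: a physics Cube pulled away from its Soutien support drives the opening of a linked BP_DoorTiming.
; While the Cube moves, Tick sends its normalized distance to the door and freezes its physics near full travel.
; While the player's Rope overlaps the Box, a looping timer adds a blocker box on the Soutien side if the Cube slides back.
; The blocker is removed on forward progress or rope release.
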(event `self.ReceiveBeginPlay`
  (`self.Get Relative Location`)
  (bind _returnvalue (`GameplayStatics.GetActorOfClass` "/Game/BP/BP_Player.BP_Player_C"))
  (set `self.PlayerRef` _returnvalue))

(event `self.ReceiveTick`
  (params (DeltaSeconds :type "Float (single-precision)"))
  (bind (_returnvalue_x _returnvalue_y _returnvalue_z) (`KismetMathLibrary.BreakVector` (`SceneComponent.GetComponentVelocity` (`self.Cube`))))
  (if (or (!= _returnvalue_x 0.0) (!= _returnvalue_y 0.0) (!= _returnvalue_z 0.0))
    (bind _relative_distance (`self.Get Relative Location`))
    (if (>= _relative_distance 195.0)
      (`PrimitiveComponent.SetSimulatePhysics` (`self.Cube`) false)
      (else
        (bind _asbp_door_timing (cast `/Game/BP/Briques_De_Jeu/BP_DoorTiming` (`self.Object to activate`)))
        (`/Game/BP/Briques_De_Jeu/BP_DoorTiming.Opening` _asbp_door_timing (`KismetMathLibrary.Abs` (`KismetMathLibrary.NormalizeToRange` (`self.Relative Distance Cube`) 0.0 200.0)))))))

(event `dont move back`
  (bind _cubebackref (`self.CubeBackRef`))
  (bind _relative_distance (`self.Get Relative Location`))
  (if (< _relative_distance (`self.LastDistance`))
    (`/Engine/EditorBlueprintResources/StandardMacros.DoOnce` false :!label _label
      (:`Completed`
        (bind _returnvalue (`AddComponent|NODE_AddBoxComponent-1`))
        (bind _output_get (set `self.CubeBackRef` _returnvalue))
        (`SceneComponent.K2_SetWorldLocation` _returnvalue (+ (`SceneComponent.K2_GetComponentLocation` (`self.Cube`)) (* (`KismetMathLibrary.GetDirectionUnitVector` (`SceneComponent.K2_GetComponentLocation` (`self.Cube`)) (`SceneComponent.K2_GetComponentLocation` (`self.Soutien`))) 255.0)) false true)
        (`SceneComponent.K2_SetWorldLocation` _output_get (+ (`SceneComponent.K2_GetComponentLocation` (`self.Cube`)) (* (`KismetMathLibrary.GetDirectionUnitVector` (`SceneComponent.K2_GetComponentLocation` (`self.Cube`)) (`SceneComponent.K2_GetComponentLocation` (`self.Soutien`))) 255.0)) false true)
        (`KismetSystemLibrary.PrintString` "Create")))
    (else
      (set `self.LastDistance` _relative_distance)
      (`/Engine/EditorBlueprintResources/StandardMacros.IsValid` _cubebackref
        (:`Is Valid`
          (`ActorComponent.K2_DestroyComponent` _cubebackref)
          (goto _label :!via `Reset`))))))

(event `self.Box.OnComponentBeginOverlap`
  (params (OverlappedComponent :type "PrimitiveComponent Object Reference") (OtherActor :type "Actor Object Reference") (OtherComp :type "PrimitiveComponent Object Reference") (OtherBodyIndex :type Integer) (bFromSweep :type Boolean) (SweepResult :type "HitResult Structure (by ref)"))
  (bind _asbp_player (cast `/Game/BP/BP_Player` OtherActor))
  (if (== (`/Game/BP/BP_Player.Rope` _asbp_player) OtherComp)
    (`/Engine/EditorBlueprintResources/StandardMacros.DoOnce` false :!label _label_2
      (:`Completed`
        (bind _returnvalue (`KismetSystemLibrary.K2_SetTimerDelegate` (delegate `dont move back`) 0.1 true))
        (set `self.move back event` _returnvalue)
        (`self.dont move back`)))))

(event `self.Box.OnComponentEndOverlap`
  (params (OverlappedComponent :type "PrimitiveComponent Object Reference") (OtherActor :type "Actor Object Reference") (OtherComp :type "PrimitiveComponent Object Reference") (OtherBodyIndex :type Integer))
  (bind _cubebackref (`self.CubeBackRef`))
  (bind _asbp_player (cast `/Game/BP/BP_Player` OtherActor))
  (if (== (`/Game/BP/BP_Player.Rope` _asbp_player) OtherComp)
    (`KismetSystemLibrary.K2_ClearAndInvalidateTimerHandle` (`self.move back event`))
    (`/Engine/EditorBlueprintResources/StandardMacros.IsValid` _cubebackref
      (:`Is Valid`
        (`ActorComponent.K2_DestroyComponent` _cubebackref)
        (set `self.LastDistance` 0.0)
        (`PrimitiveComponent.SetSimulatePhysics` (`self.Cube`) true)
        (`|ExecutionSequence`
          (:`then_0`
            (goto _label_2 :!via `Reset`))
          (:`then_1`
            (goto _label :!via `Reset`)))))))

(fn `Get Relative Location`
  (returns (`relative distance` :type "Float (double-precision)"))
  (bind _output_get (set `self.Relative Distance Cube` (- (`KismetMathLibrary.Vector_Distance` (`SceneComponent.K2_GetComponentLocation` (`self.Cube`)) (`SceneComponent.K2_GetComponentLocation` (`self.Soutien`))) 255.0)))
  (return _output_get))

(fn `UserConstructionScript`)