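; BP_Tirolienne is a zipline hook that rides along a spline and destroys itself at the end.
; Move drives a timeline scaled to the travel time, setting location and yaw from spline distance.
; Its Box detects the player's Rope, notifies the player on enter and exit, and registers itself with its BP_SplinePathTyrolienne on enter.
; StopCollide shakes the camera and disables the hook's collision for a second.
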(event `self.ReceiveBeginPlay`
  (bind _asbp_player (cast `/Game/BP/BP_Player` (`GameplayStatics.GetPlayerPawn` 0)))
  (set `self.As BP Player` _asbp_player))

(event `Move`
  (params (Spline :type "SplineComponent Object Reference") (`Time To travel` :type "Float (double-precision)") (BP_spline :type "Actor Object Reference"))
  (set `self.BP SplineRef` BP_spline)
  (`TimelineComponent.SetPlayRate` (`self.MoveTimeline`) (/ 1.0 `Time To travel`))
  (bind (_direction _newtrack_0) (`Timeline|MoveTimeline` :!via `PlayFromStart`)
    (:`Update`
      (bind _returnvalue (`KismetMathLibrary.Lerp` 0.0 (`SplineComponent.GetSplineLength` Spline) _newtrack_0))
      (bind (_returnvalue_roll _returnvalue_pitch _returnvalue_yaw) (`KismetMathLibrary.BreakRotator` (`SplineComponent.GetRotationAtDistanceAlongSpline` Spline _returnvalue "Local")))
      (`self.K2_SetActorTransform` (`KismetMathLibrary.MakeTransform` (`SplineComponent.GetLocationAtDistanceAlongSpline` Spline _returnvalue "World") (`KismetMathLibrary.MakeRotator` 0.0 0.0 _returnvalue_yaw))))
    (:`Finished`
      (`self.End Course`))))

(event `End Course`
  (`self.K2_DestroyActor`))

(event `self.Box.OnComponentBeginOverlap`
  (params (OverlappedComponent :type "PrimitiveComponent Object Reference") (OtherActor :type "Actor Object Reference") (OtherComp :type "PrimitiveComponent Object Reference") (OtherBodyIndex :type Integer) (bFromSweep :type Boolean) (SweepResult :type "HitResult Structure (by ref)"))
  (if (== (`/Game/BP/BP_Player.Rope` (`self.As BP Player`)) OtherComp)
    (`KismetSystemLibrary.PrintString` "Jrentre en overlappe")
    (`/Game/BP/BP_Player.OverlappingTyro` (`self.As BP Player`))
    (bind _asbp_spline_path_tyrolienne (cast `/Game/BP/Briques_De_Jeu/BP_SplinePathTyrolienne` (`self.BP SplineRef`)))
    (`/Game/BP/Briques_De_Jeu/BP_SplinePathTyrolienne.GetTyroRef` _asbp_spline_path_tyrolienne self)))

(event `self.Box.OnComponentEndOverlap`
  (params (OverlappedComponent :type "PrimitiveComponent Object Reference") (OtherActor :type "Actor Object Reference") (OtherComp :type "PrimitiveComponent Object Reference") (OtherBodyIndex :type Integer))
  (if (== (`/Game/BP/BP_Player.Rope` (`self.As BP Player`)) OtherComp)
    (`KismetSystemLibrary.PrintString` "Jsors de l'overlappe")
    (`/Game/BP/BP_Player.EndOverlap` (`self.As BP Player`))))

(event `StopCollide`
  (`PrimitiveComponent.SetCollisionEnabled` (`self.crochet_rond_Physics`) "NoCollision")
  (`PlayerCameraManager.StartCameraShake` :`self` (`GameplayStatics.GetPlayerCameraManager` 0) :`ShakeClass` "/Game/FirstPerson/CameraShake/MachineShake.MachineShake_C")
  (`KismetSystemLibrary.Delay` 1.0)
  (`PrimitiveComponent.SetCollisionEnabled` (`self.crochet_rond_Physics`) "QueryAndPhysics"))

(fn `UserConstructionScript`)