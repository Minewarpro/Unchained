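; BP_Ladder is a ladder gameplay actor that tells the player when it enters or leaves the ladder.
; Begin overlap on the Hit component calls OnLadder on BP_Player, while end overlap on a separate Box component calls OutLadder.
; Both events respond only when the overlapping component is the player's capsule, leaving the ladder behavior itself to BP_Player.
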(event `self.Hit.OnComponentBeginOverlap`
  (params (OverlappedComponent :type "PrimitiveComponent Object Reference") (OtherActor :type "Actor Object Reference") (OtherComp :type "PrimitiveComponent Object Reference") (OtherBodyIndex :type Integer) (bFromSweep :type Boolean) (SweepResult :type "HitResult Structure (by ref)"))
  (bind _asbp_player (cast `/Game/BP/BP_Player` OtherActor))
  (if (== (`/Game/BP/BP_Player.Capsule` _asbp_player) OtherComp)
    (`/Game/BP/BP_Player.OnLadder` _asbp_player)))

(event `self.Box.OnComponentEndOverlap`
  (params (OverlappedComponent :type "PrimitiveComponent Object Reference") (OtherActor :type "Actor Object Reference") (OtherComp :type "PrimitiveComponent Object Reference") (OtherBodyIndex :type Integer))
  (bind _asbp_player (cast `/Game/BP/BP_Player` OtherActor))
  (if (== (`/Game/BP/BP_Player.Capsule` _asbp_player) OtherComp)
    (`/Game/BP/BP_Player.OutLadder` _asbp_player)))

(fn `UserConstructionScript`)