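; BP_BreakablePlank is a Chaos Geometry Collection plank that fades through a material Alpha parameter and destroys itself once broken.
; The construction script creates one dynamic material instance and assigns it to every material slot.
; The first break event sets collision to ignore pawns and two custom channels, then plays a timeline.
; The timeline drives Alpha through ChangeMaterial, which also reapplies the material, and destroys the actor when finished.
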(event `self.Plank.OnChaosBreakEvent`
  (params (BreakEvent :type "ChaosBreakEvent Structure (by ref)"))
  (`/Engine/EditorBlueprintResources/StandardMacros.DoOnce` false
    (:`Completed`
      ;[0.07812 0.07812 0.07812] Set Collision Response
      (`PrimitiveComponent.SetCollisionResponseToChannel` (`self.Plank`) "ECC_GameTraceChannel5" "ECR_Ignore")
      (`PrimitiveComponent.SetCollisionResponseToChannel` (`self.GeometryCollectionComponent`) "ECC_GameTraceChannel5" "ECR_Ignore")
      (`PrimitiveComponent.SetCollisionResponseToChannel` (`self.Plank`) "ECC_GameTraceChannel6" "ECR_Ignore")
      (`PrimitiveComponent.SetCollisionResponseToChannel` (`self.GeometryCollectionComponent`) "ECC_GameTraceChannel6" "ECR_Ignore")
      (`PrimitiveComponent.SetCollisionResponseToChannel` (`self.Plank`) "ECC_Pawn" "ECR_Ignore")
      (`PrimitiveComponent.SetCollisionResponseToChannel` (`self.GeometryCollectionComponent`) "ECC_Pawn" "ECR_Ignore")
      ;[0.09375 0.09375 0.09375] Set Alpha And Destroy
      (bind (_direction _newtrack_0) (`Timeline|Timeline`)
        (:`Update`
          (`self.ChangeMaterial` _newtrack_0))
        (:`Finished`
          (`self.K2_DestroyActor`))))))

(fn `ChangeMaterial`
  (params (TimeLineAlpha :type "Float (double-precision)"))
  (`MaterialInstanceDynamic.SetScalarParameterValue` (`self.MaterialInstance`) "Alpha" TimeLineAlpha)
  (for (_ _array_index) (`MeshComponent.GetMaterials` (`self.Plank`))
    (`PrimitiveComponent.SetMaterial` (`self.Plank`) _array_index (`self.MaterialInstance`))))

(fn `UserConstructionScript`
  (bind _plank (`self.Plank`))
  (bind _returnvalue (`PrimitiveComponent.CreateDynamicMaterialInstance` _plank 0 "/Game/Materials/M_PlankTEst.M_PlankTEst" "None"))
  (bind _output_get (set `self.MaterialInstance` _returnvalue))
  (for (_ _array_index) (`MeshComponent.GetMaterials` _plank)
    (`PrimitiveComponent.SetMaterial` (`self.Plank`) _array_index _output_get)))