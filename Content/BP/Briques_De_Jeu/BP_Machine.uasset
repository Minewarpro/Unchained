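; BP_Machine is a looping piston machine that can blow up the player's Boulet.
; It starts once, when activation calls bring its active-object count to the required number.
; A slowed timeline drives the piston along Z and restarts itself, with a swoosh each cycle and a metal impact near full extension.
; A piston hit while the Boulet is inside the trigger box calls ExplosionBoulet on BP_Player, once only.
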(event `self.ReceiveBeginPlay`
  (`TimelineComponent.SetPlayRate` (`self.PistonMove`) 0.3))

(event `StartMachine`
  (`GameplayStatics.PlaySoundAtLocation` "/Game/SFX/Environnement/Cue_BigSwoosh.Cue_BigSwoosh" (`self.K2_GetActorLocation`) (struct) 1.0 1.0 0.0 null null null null)
  (bind (_direction _newtrack_0) (`Timeline|PistonMove` :!via `PlayFromStart`)
    (:`Update`
      (`SceneComponent.K2_SetRelativeLocation` (`self.Piston`) (`KismetMathLibrary.MakeVector` 0.0 0.0 (* _newtrack_0 -190.0)) false false)
      (if (>= _newtrack_0 0.9)
        (`/Engine/EditorBlueprintResources/StandardMacros.DoOnce` false :!label _label
          (:`Completed`
            (`GameplayStatics.PlaySoundAtLocation` "/Game/SFX/Environnement/Cue_MetalImpact.Cue_MetalImpact" (`self.K2_GetActorLocation`) (struct) 1.0 1.0 0.0 null null null null)))))
    (:`Finished`
      (`self.StartMachine`)
      (goto _label :!via `Reset`))))

(event `/Game/BP/Briques_De_Jeu/BPI_ActivateObject.ActivateObject`
  (bind _output_get (set `self.ObjectActiveCurrent` (+ (`self.ObjectActiveCurrent`) 1)))
  (if (== _output_get (`self.ObjectActiveNb`))
    (`/Engine/EditorBlueprintResources/StandardMacros.DoOnce` false
      (:`Completed`
        (`self.StartMachine`)))))

(event `/Game/BP/Briques_De_Jeu/BPI_DesactivateObject.DesactivateObject`
  (set `self.ObjectActiveCurrent` (- (`self.ObjectActiveCurrent`) 1)))

(event `self.Box.OnComponentBeginOverlap`
  (params (OverlappedComponent :type "PrimitiveComponent Object Reference") (OtherActor :type "Actor Object Reference") (OtherComp :type "PrimitiveComponent Object Reference") (OtherBodyIndex :type Integer) (bFromSweep :type Boolean) (SweepResult :type "HitResult Structure (by ref)"))
  (bind _asbp_player (cast `/Game/BP/BP_Player` OtherActor))
  (if (== (`/Game/BP/BP_Player.Boulet` _asbp_player) OtherComp)
    (set `self.Boulet Overlap` true)))

(event `self.Box.OnComponentEndOverlap`
  (params (OverlappedComponent :type "PrimitiveComponent Object Reference") (OtherActor :type "Actor Object Reference") (OtherComp :type "PrimitiveComponent Object Reference") (OtherBodyIndex :type Integer))
  (bind _asbp_player (cast `/Game/BP/BP_Player` OtherActor))
  (if (== (`/Game/BP/BP_Player.Boulet` _asbp_player) OtherComp)
    (set `self.Boulet Overlap` false)))

(event `self.Piston.OnComponentHit`
  (params (HitComponent :type "PrimitiveComponent Object Reference") (OtherActor :type "Actor Object Reference") (OtherComp :type "PrimitiveComponent Object Reference") (NormalImpulse :type "Vector Structure") (Hit :type "HitResult Structure (by ref)"))
  (bind _asbp_player (cast `/Game/BP/BP_Player` OtherActor))
  (if (and (== (`/Game/BP/BP_Player.Boulet` _asbp_player) OtherComp) (`self.Boulet Overlap`))
    (`/Engine/EditorBlueprintResources/StandardMacros.DoOnce` false
      (:`Completed`
        (`KismetSystemLibrary.PrintString` "Explosion")
        (bind _asbp_player_2 (cast `/Game/BP/BP_Player` OtherActor))
        (`/Game/BP/BP_Player.ExplosionBoulet` _asbp_player_2)))))

(fn `UserConstructionScript`)