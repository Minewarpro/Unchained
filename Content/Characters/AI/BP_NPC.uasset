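; BP_NPC is an AI character that varies its walk speed by distance to the player and can respawn at its starting location.
; A looping timer randomly picks fast or slow speed when the player is far away, otherwise slow.
; Tick forces slow speed when the player is near and prints the speed for debugging.
; It hides its rock mesh at BeginPlay, with an event to toggle it.
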(event `SetRockVisible`
  (params (Hidden :type Boolean))
  (`SceneComponent.SetHiddenInGame` (`self.StaticMesh`) Hidden false))

(event `self.ReceiveBeginPlay`
  (`KismetSystemLibrary.K2_SetTimerDelegate` (delegate `RandomSpeed`) 5.0 true)
  (set `self.InitialPosition` (`self.K2_GetActorLocation`))
  (`self.SetRockVisible` true))

(event `Respawn`
  (`self.K2_SetActorLocation` (`self.InitialPosition`) false true)
  (`self.K2_SetActorRotation` (struct)))

(event `RandomSpeed`
  (bind _charactermovement (`self.CharacterMovement`))
  (if (> (`self.GetDistanceTo` (`GameplayStatics.GetPlayerPawn` 0)) 1000.0)
    (if (< (`KismetMathLibrary.RandomIntegerInRange` 1 100) 50)
      (set `CharacterMovementComponent.MaxWalkSpeed` 400.0 _charactermovement)
      (else
        (set `CharacterMovementComponent.MaxWalkSpeed` 200.0 _charactermovement :!label _label)))
    (else
      (goto _label))))

(event `self.ReceiveTick`
  (params (DeltaSeconds :type "Float (single-precision)"))
  (bind _maxwalkspeed (`CharacterMovementComponent.MaxWalkSpeed` (`self.CharacterMovement`)))
  (`KismetSystemLibrary.PrintString` (`KismetStringLibrary.Conv_DoubleToString` _maxwalkspeed) true true (struct :`G` 0.66 :`B` 1.0 :`A` 1.0) 0.0)
  (if (and (< (`self.GetDistanceTo` (`GameplayStatics.GetPlayerPawn` 0)) 1000.0) (!= _maxwalkspeed 200.0))
    (set `CharacterMovementComponent.MaxWalkSpeed` 200.0 (`self.CharacterMovement`))))

(fn `UserConstructionScript`)